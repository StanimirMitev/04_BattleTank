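; Player-controlled tank Blueprint that binds input to driving, camera aiming and firing.
; On BeginPlay it registers the Barrel and Turret and initialises the TankMove component with the left and right tracks.
; Aim axes rotate a separate azimuth gimbal for yaw and the spring arm for pitch.
; Drive and turn axes forward intent to TankMove, and the Fire action calls Fire.
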(event `self.ReceiveBeginPlay`
  (`self.SetBarrelReference` (`self.Barrel`))
  (`self.SetTurretReference` (`self.Turret`))
  (`TankMovementComponent.Initialise` (`self.TankMove`) (`self.Track_Right`) (`self.Track_Left`)))

(event `InputAxis|AimAltitude`
  (params (AxisValue :type "Float (single-precision)"))
  ;[1 1 1] Aiming Stuff
  (`SceneComponent.K2_AddLocalRotation` (`self.SpringArm`) (`KismetMathLibrary.MakeRotator` 0.0 AxisValue) false false))

(event `InputAxis|MoveForWard`
  (params (AxisValue :type "Float (single-precision)"))
  (`TankMovementComponent.IntendMoveForward` (`self.TankMove`) AxisValue))

(event `InputAxis|MoveBackward`
  (params (AxisValue :type "Float (single-precision)"))
  (`TankMovementComponent.IntendMoveForward` (`self.TankMove`) AxisValue))

(event `InputAxis|AimAzimuth`
  (params (AxisValue :type "Float (single-precision)"))
  ;[1 1 1] Aiming Stuff
  (`SceneComponent.K2_AddLocalRotation` (`self.Azimut Gimbal`) (`KismetMathLibrary.MakeRotator` 0.0 0.0 AxisValue) false false))

(event `InputAxis|TurnRight`
  (params (AxisValue :type "Float (single-precision)"))
  (`TankMovementComponent.IntendTurn` (`self.TankMove`) AxisValue))

(event `InputAxis|TurnLeft`
  (params (AxisValue :type "Float (single-precision)"))
  (`TankMovementComponent.IntendTurn` (`self.TankMove`) AxisValue))

(event `InputAction|Fire`
  (params (Key :type "Key Structure"))
  ;[1 1 1] Aiming Stuff
  (:`Pressed`
    (`self.Fire`)))

(fn `UserConstructionScript`)